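; Base enemy character for a side-scroller, providing patrol, chase, damage and knockback behavior along the X axis.
; Patrolling moves around the construction-time start point with random pauses and turns, while PawnSensing sets a chase flag that clears beyond a distance threshold.
; Hitting Bob launches both apart and damages him; damage taken spawns random sparks, updates the health widget and destroys at zero.
; Movement routines, hovering included, have no caller here.
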(event `TurnAround`
  ;[0 0.1336 1] Movement
  ;;[1 0.526 0.526] TurnAround
  (`SceneComponent.K2_SetRelativeRotation` (`self.CapsuleComponent`) (`KismetMathLibrary.MakeRotator` 0.0 0.0 (`KismetMathLibrary.SelectFloat` 0.0 180.0 (`self.IsMovingRight `))) false false)
  (`SceneComponent.K2_SetWorldRotation` (`self.Widget`) (struct :`Yaw` 90.0) false false))

(event `RandomChoice`
  ;[0 0.1336 1] Movement
  ;;[1 0.526 0.526] Entscheidungen beim Patrollieren (umdrehen, stehenbleiben)
  (if (== (`KismetMathLibrary.RandomInteger` 1000) 0)
    (set `self.Pausing` true)
    (`KismetSystemLibrary.Delay` 3.0)
    (set `self.Pausing` false)
    (if (== (`KismetMathLibrary.RandomInteger` 2) 0)
      (if (`self.IsMovingRight `)
        (set `self.IsMovingRight ` false)
        (else
          (set `self.IsMovingRight ` true)))
      (`self.TurnAround`))))

(event `changeHealth`
  ;[1 0.08854 0.08854] Grundfunktionen
  ;;[0.6565 1 0.555] Change Health
  (bind _asenemy_health (cast `/Game/Blueprints/Enemies/EnemyHealth` (`WidgetComponent.GetUserWidgetObject` (`self.Widget`))))
  (`ProgressBar.SetPercent` (`/Game/Blueprints/Enemies/EnemyHealth.ProgressBar_0` _asenemy_health) (/ (`self.Health`) (`self.Max Health`)))
  (if (<= (`self.Health`) 0.0)
    (`self.K2_DestroyActor`)))

(event `self.ReceiveAnyDamage`
  (params (Damage :type "Float (single-precision)") (DamageType :type "DamageType Object Reference") (InstigatedBy :type "Controller Object Reference") (DamageCauser :type "Actor Object Reference"))
  ;[1 0.08854 0.08854] Grundfunktionen
  ;;[0.6565 1 0.555] Get Damage
  (`self.HitSpark`)
  (set `self.Health` (- (`self.Health`) Damage))
  (`self.changeHealth`))

(event `self.CapsuleComponent.OnComponentHit`
  (params (HitComponent :type "PrimitiveComponent Object Reference") (OtherActor :type "Actor Object Reference") (OtherComp :type "PrimitiveComponent Object Reference") (NormalImpulse :type "Vector Structure") (Hit :type "HitResult Structure (by ref)"))
  (bind _returnvalue_x (`KismetMathLibrary.BreakVector` (`self.K2_GetActorLocation`)))
  ;[1 0.08854 0.08854] Grundfunktionen
  ;;[1 0.7036 0.4121] Bob knockback
  (bind _asbob (cast `/Game/Blueprints/Bob/Bob` OtherActor))
  (bind _returnvalue_x_2 (`KismetMathLibrary.BreakVector` (`self.K2_GetActorLocation` _asbob)))
  (if (<= _returnvalue_x_2 _returnvalue_x)
    (`self.LaunchCharacter` _asbob (-500.0 0.0 300.0) true true)
    (`self.LaunchCharacter` (500.0 0.0 300.0) true true)
    (else
      (`self.LaunchCharacter` _asbob (500.0 0.0 300.0) true true)
      (`self.LaunchCharacter` (-500.0 0.0 300.0) true true)))
  (`GameplayStatics.ApplyDamage` _asbob (`self.Damage`)))

(event `Patroll`
  (bind _returnvalue_x (`KismetMathLibrary.BreakVector` (`self.K2_GetActorLocation`)))
  (bind _patroldistance (`self.PatrolDistance`))
  (bind _startpoint_x (`KismetMathLibrary.BreakVector` (`self.StartPoint`)))
  ;[0 0.1336 1] Movement
  ;;[0.6565 1 0.555] Patrolling
  (`|ExecutionSequence`
    (:`then_0`
      (`/Engine/EditorBlueprintResources/StandardMacros.DoOnce` false
        (:`Completed`
          (`self.TurnAround`))))
    (:`then_1`
      (if (`self.Pausing`)
        _
        (elif (`self.IsMovingRight `)
          (`self.AddMovementInput` (9999.0 0.0 0.0))
          (`self.RandomChoice`)
          (if (>= _returnvalue_x (+ _startpoint_x _patroldistance))
            (set `self.Pausing` true)
            (`KismetSystemLibrary.Delay` 2.0)
            (set `self.Pausing` false)
            (set `self.IsMovingRight ` false)
            (`self.TurnAround` :!label _label))
          (else
            (`self.AddMovementInput` (-9999.0 0.0 0.0))
            (`self.RandomChoice`)
            (if (<= _returnvalue_x (- _startpoint_x _patroldistance))
              (set `self.Pausing` true)
              (`KismetSystemLibrary.Delay` 2.0)
              (set `self.Pausing` false)
              (set `self.IsMovingRight ` true)
              (goto _label))))))))

(event `CalculateDistance`
  (bind _returnvalue_x (`KismetMathLibrary.BreakVector` (`self.K2_GetActorLocation`)))
  (bind _returnvalue_x_2 (`KismetMathLibrary.BreakVector` (`self.K2_GetActorLocation` (`GameplayStatics.GetPlayerCharacter` 0))))
  (bind _returnvalue (- _returnvalue_x _returnvalue_x_2))
  ;[1 0.08854 0.08854] Grundfunktionen
  ;;[0.4479 0.5155 1] Distanz zu Bob
  (if (>= _returnvalue 0.0)
    (set `self.Distance` _returnvalue)
    (else
      (set `self.Distance` (* -1 _returnvalue)))))

(event `self.PawnSensing.OnSeePawn`
  (params (Pawn :type "Pawn Object Reference"))
  ;[1 0.08854 0.08854] Grundfunktionen
  ;;[0.4479 0.5155 1] Start Chase
  (set `self.Chasing` true))

(event `Chase`
  (bind _returnvalue_x (`KismetMathLibrary.BreakVector` (`KismetMathLibrary.Normal` (- (`self.K2_GetActorLocation` (`GameplayStatics.GetPlayerCharacter` 0)) (`self.K2_GetActorLocation`)))))
  ;[0 0.1336 1] Movement
  ;;[0.6565 1 0.555] Chasing
  (if (not (`self.Attacking`))
    (if (> _returnvalue_x 0.0)
      (set `self.IsMovingRight ` true)
      (else
        (set `self.IsMovingRight ` false)))
    (`self.AddMovementInput` (`KismetMathLibrary.MakeVector` _returnvalue_x))
    (`self.TurnAround`)
    (`self.StopChase`)))

(event `self.OnLanded`
  (params (Hit :type "HitResult Structure (by ref)"))
  ;[1 0.08854 0.08854] Grundfunktionen
  (if (`self.GetFallDamage`)
    (`self.GetFallDmg` (`self.Float`))))

(event `HitSpark`
  (bind _returnvalue (`self.K2_GetActorLocation`))
  (bind _returnvalue_2 (`self.K2_GetActorRotation`))
  ;[1 0.08854 0.08854] Grundfunktionen
  ;;[0 0 0] Hitsparks
  (switch `int` (`KismetMathLibrary.RandomInteger` 5)
    (:`0`
      (`GameplayStatics.SpawnEmitterAtLocation` "/Game/InfinityBladeEffects/Effects/HitSparkBob1.HitSparkBob1" _returnvalue _returnvalue_2))
    (:`1`
      (`GameplayStatics.SpawnEmitterAtLocation` "/Game/InfinityBladeEffects/Effects/HitSparkBob3.HitSparkBob3" _returnvalue _returnvalue_2))
    (:`2`
      (`GameplayStatics.SpawnEmitterAtLocation` "/Game/InfinityBladeEffects/Effects/HitSparkBob5.HitSparkBob5" _returnvalue _returnvalue_2))
    (:`3`
      (`GameplayStatics.SpawnEmitterAtLocation` "/Game/InfinityBladeEffects/Effects/HitSparkBoB4.HitSparkBoB4" _returnvalue _returnvalue_2))
    (:`4`
      (`GameplayStatics.SpawnEmitterAtLocation` "/Game/InfinityBladeEffects/Effects/HitSparkBob2.HitSparkBob2" _returnvalue _returnvalue_2))))

(event `StopChase`
  ;[0 0.1336 1] Movement
  ;;[0.6565 1 0.555] Stop Chasing
  (if (>= (`self.Distance`) 1000.0)
    (set `self.Chasing` false)))

(event `FlyingUpAndDown`
  (bind (_returnvalue_x _returnvalue_y _returnvalue_z) (`KismetMathLibrary.BreakVector` (`self.K2_GetActorLocation`)))
  (bind (_startpoint_x _startpoint_y _startpoint_z) (`KismetMathLibrary.BreakVector` (`self.StartPoint`)))
  ;[0 0.1336 1] Movement
  ;;[0.6565 1 0.555] Flying Up And Down
  (if (<= _returnvalue_z _startpoint_z)
    (`self.AddMovementInput` (0.0 0.0 10.0))
    (else
      (`self.AddMovementInput` (0.0 0.0 -10.0)))))

(fn `GetFallDmg`
  (params (Dmg :type "Float (double-precision)"))
  (set `self.Health` (- (`self.Health`) Dmg))
  (`self.changeHealth`))

(fn `SetupFallDmg`
  (params (dm :type "Float (double-precision)"))
  (set `self.Float` dm)
  (set `self.GetFallDamage` true))

(fn `UserConstructionScript`
  (set `self.StartPoint` (`self.K2_GetActorLocation`)))