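; Side-scrolling Rusher enemy that patrols between two points, activating on heard noise and switching to chase on sight.
; Construction script feeds PointA/PointB into InterpToMovement, whose reversals flip the sprite.
; Tick derives an Idle/Patrolling/Chasing/Attacking enum from boolean flags and drives Chase, whose direction subtracts two actor locations.
; Attack tilts and launches the character sideways with a slam sound, but its only caller, a range check, is disconnected.
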(event `Attack`
  ;[1 1 1] Attack
  (set `self.Attacking_0` true)
  (`ActorComponent.ToggleActive` (`self.InterpToMovement_0`))
  (`self.K2_AddActorLocalRotation` (struct :`Pitch` -45.0))
  (`KismetSystemLibrary.Delay` 0.5)
  (`GameplayStatics.SpawnSoundAttached` "/Game/Sounds/NFF-slam.NFF-slam" (`self.CapsuleComponent`) "None" (0.0 0.0 0.0) (struct) "KeepRelativeOffset" false 0.6 2.0)
  (`self.LaunchCharacter` (`KismetMathLibrary.SelectVector` (-3000.0 0.0 0.0) (3000.0 0.0 0.0) (`self.IsMovingLeft`)))
  (`KismetSystemLibrary.Delay` 1.0)
  (`self.K2_AddActorLocalRotation` (struct :`Pitch` 45.0))
  (set `self.Attacking_0` false)
  (`self.Chase`))

(event `self.ReceiveTick`
  (params (DeltaSeconds :type "Float (single-precision)"))
  ;[1 1 1] Statehandler
  (`|ExecutionSequence`
    (:`then_1`
      (if (`self.InRange`)
        (if (`self.Chasing_0`)
          (if (`self.Attacking_0`)
            (set `self.EnemyStateEnum_0` "NewEnumerator3")
            (else
              (set `self.EnemyStateEnum_0` "NewEnumerator2")))
          (else
            (set `self.EnemyStateEnum_0` "NewEnumerator1")))
        (else
          (set `self.EnemyStateEnum_0` "NewEnumerator0"))))
    (:`then_2`
      (switch `/Game/Blueprints/Enemies/EnemyState` (`self.EnemyStateEnum_0`)
        (:`NewEnumerator0`
          (set `self.InRange` false))
        (:`NewEnumerator1`
          (set `self.InRange` true))
        (:`NewEnumerator2`
          (set `self.Chasing_0` true))
        (:`NewEnumerator3`
          (set `self.Attacking_0` true))))
    (:`then_3`
      (if (`self.Chasing_0`)
        (if (not (`self.Attacking_0`))
          (`self.Chase`))))))

(event `Activate Enemy`
  ;[1 1 1] Enemy Rotation wenn Punkt A oder B erreicht wird
)

(event `self.InterpToMovement_0.OnInterpToReverse`
  (params (ImpactResult :type "HitResult Structure (by ref)") (Time :type "Float (single-precision)"))
  ;[1 1 1] Enemy Rotation wenn Punkt A oder B erreicht wird
  (if (`self.IsMovingLeft`)
    (set `self.IsMovingLeft` false)
    (else
      (set `self.IsMovingLeft` true)))
  (`SceneComponent.K2_SetRelativeRotation` (`self.Sprite`) (`KismetMathLibrary.MakeRotator` 0.0 0.0 (`KismetMathLibrary.SelectFloat` 0.0 180.0 (`self.IsMovingLeft`))) false false))

(event `self.PawnSensing.OnSeePawn`
  (params (Pawn :type "Pawn Object Reference"))
  ;[1 1 1] Rusher startet seinen Angriff, wenn wir in see-range sind
  (set `self.Chasing_0` true))

(event `Chase`
  ;[1 1 1] Verfolgen nach dem Angriff
  (set `self.Chasing_0` true)
  (`self.AddMovementInput` (`KismetMathLibrary.Normal` (- (`self.K2_GetActorLocation`) (`self.K2_GetActorLocation`)))))

(event `self.PawnSensing.OnHearNoise`
  (params (Instigator :type "Pawn Object Reference") (Location :type "Vector Structure (by ref)") (Volume :type "Float (single-precision)"))
  (bind _returnvalue_x (`KismetMathLibrary.BreakVector` (`self.K2_GetActorLocation`)))
  (bind _returnvalue_x_2 (`KismetMathLibrary.BreakVector` (`self.K2_GetActorLocation`)))
  ;[1 1 1] Rusher wird erst aktiv, wenn wir in hear-range sind
  (set `self.Distance_0` (- _returnvalue_x_2 _returnvalue_x))
  (if (not (`self.Chasing_0`))
    (`ActorComponent.SetActive` (`self.InterpToMovement_0`) true true)
    (set `self.InRange` true)))

(fn `UserConstructionScript`
  (set `InterpToMovementComponent.ControlPoints` (`|MakeArray` (make `InterpControlPoint` (`self.pointA`)) (make `InterpControlPoint` (`self.pointB`))) (`self.InterpToMovement_0`)))