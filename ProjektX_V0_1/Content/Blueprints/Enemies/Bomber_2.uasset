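; Bomber_2 is an enemy Blueprint with health, damage handling and two-stage pawn sensing, apparently an unfinished variant of a Rusher.
; Tick updates the health bar widget and destroys the actor at zero health, which AnyDamage and GetDamaged reduce.
; Hearing sets InRange so Tick calls ActivateEnemy, while seeing calls Attack and blocks reactivation.
; ActivateEnemy and Attack are empty; shooting, knockback, patrol and chase logic is disconnected.
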(event `self.ReceiveTick`
  (params (DeltaSeconds :type "Float (single-precision)"))
  (`|ExecutionSequence`
    (:`then_0`
      (bind _asenemy_health (cast `/Game/Blueprints/Enemies/EnemyHealth` (`WidgetComponent.GetUserWidgetObject` (`self.EnemyHealthUI`))))
      (`ProgressBar.SetPercent` (`/Game/Blueprints/Enemies/EnemyHealth.ProgressBar_0` _asenemy_health) (/ (`self.Health`) 100.0))
      (if (<= (`self.Health`) 0.0)
        (`self.K2_DestroyActor`)))
    (:`then_1`
      (if (`self.InRange`)
        (`self.Activate Enemy`)))))

(event `self.ReceiveAnyDamage`
  (params (Damage :type "Float (single-precision)") (DamageType :type "DamageType Object Reference") (InstigatedBy :type "Controller Object Reference") (DamageCauser :type "Actor Object Reference"))
  (set `self.Health` (- (`self.Health`) Damage)))

(event `GetDamaged`
  (params (DmgIn :type "Float (double-precision)"))
  (set `self.Health` (- (`self.Health`) DmgIn)))

(event `self.CapsuleComponent.OnComponentHit`
  (params (HitComponent :type "PrimitiveComponent Object Reference") (OtherActor :type "Actor Object Reference") (OtherComp :type "PrimitiveComponent Object Reference") (NormalImpulse :type "Vector Structure") (Hit :type "HitResult Structure (by ref)")))

(event `Attack`
  ;[1 1 1] Attack
)

(event `self.PawnSensing.OnSeePawn`
  (params (Pawn :type "Pawn Object Reference"))
  ;[1 1 1] Rusher startet seinen Angriff, wenn wir in see-range sind
  (`KismetSystemLibrary.PrintString` "seeing")
  (`self.Attack`)
  (set `self.InRange` false)
  (set `self.Attacking` true))

(event `Activate Enemy`
  ;[1 1 1] Enemy Movement
)

(event `self.PawnSensing.OnHearNoise`
  (params (Instigator :type "Pawn Object Reference") (Location :type "Vector Structure (by ref)") (Volume :type "Float (single-precision)"))
  ;[1 1 1] Rusher wird erst aktiv, wenn wir in hear-range sind
  (if (not (`self.Attacking`))
    (`KismetSystemLibrary.PrintString` "hearing")
    (set `self.InRange` true)))

(fn `UserConstructionScript`)