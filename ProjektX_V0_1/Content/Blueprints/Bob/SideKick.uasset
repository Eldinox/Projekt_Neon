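; SideKick is a flying companion character that follows the player in the X/Z plane, hovering above them and offset to whichever side it is currently on.
; Each Tick switches max fly speed by horizontal distance, recalculates that distance, then steers toward the offset point with normalized movement input.
; Input strength scales with distance outside a comfort band and drops to a gentle constant drift inside it.
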(event `CalculateDistance`
  (bind _returnvalue_x (`KismetMathLibrary.BreakVector` (`self.K2_GetActorLocation`)))
  (bind _returnvalue_x_2 (`KismetMathLibrary.BreakVector` (`self.K2_GetActorLocation` (`GameplayStatics.GetPlayerCharacter` 0))))
  (bind _returnvalue (- _returnvalue_x _returnvalue_x_2))
  (if (>= _returnvalue 0.0)
    (set `self.Distance` _returnvalue)
    (else
      (set `self.Distance` (* -1 _returnvalue)))))

(event `self.ReceiveTick`
  (params (DeltaSeconds :type "Float (single-precision)"))
  (bind _returnvalue_x (`KismetMathLibrary.BreakVector` (`self.K2_GetActorLocation`)))
  (bind _charactermovement (`self.CharacterMovement`))
  (bind _returnvalue_x_2 (`KismetMathLibrary.BreakVector` (`self.K2_GetActorLocation` (`GameplayStatics.GetPlayerCharacter` 0))))
  (bind (_returnvalue_x_3 _returnvalue_y _returnvalue_z) (`KismetMathLibrary.BreakVector` (- (`self.K2_GetActorLocation` (`GameplayStatics.GetPlayerCharacter` 0)) (`self.K2_GetActorLocation`))))
  (bind (_returnvalue_x_4 _returnvalue_y_2 _returnvalue_z_2) (`KismetMathLibrary.BreakVector` (- (`self.K2_GetActorLocation` (`GameplayStatics.GetPlayerCharacter` 0)) (`self.K2_GetActorLocation`))))
  (bind (_returnvalue_x_5 _returnvalue_y_3 _returnvalue_z_3) (`KismetMathLibrary.BreakVector` (`KismetMathLibrary.Normal` (`KismetMathLibrary.MakeVector` (- _returnvalue_x_3 -200.0) 0.0 (+ _returnvalue_z 100.0)))))
  (bind (_returnvalue_x_6 _returnvalue_y_4 _returnvalue_z_4) (`KismetMathLibrary.BreakVector` (`KismetMathLibrary.Normal` (`KismetMathLibrary.MakeVector` (- _returnvalue_x_4 200.0) 0.0 (+ _returnvalue_z_2 100.0)))))
  (`|ExecutionSequence`
    (:`then_0`
      (if (>= (`self.Distance`) 600.0)
        (set `CharacterMovementComponent.MaxFlySpeed` 600.0 _charactermovement)
        (else
          (set `CharacterMovementComponent.MaxFlySpeed` 300.0 _charactermovement))))
    (:`then_1`
      (`self.CalculateDistance`)
      (if (>= _returnvalue_x_2 _returnvalue_x)
        (if (or (>= (`self.Distance`) 250.0) (<= (`self.Distance`) 150.0))
          (`self.AddMovementInput` (`KismetMathLibrary.MakeVector` _returnvalue_x_6 0.0 _returnvalue_z_4) (* 3 (* (`self.Distance`) 0.001)))
          (else
            (`self.AddMovementInput` (`KismetMathLibrary.MakeVector` _returnvalue_x_6 0.0 _returnvalue_z_4) 0.1)))
        (elif (or (>= (`self.Distance`) 250.0) (<= (`self.Distance`) 150.0))
          (`self.AddMovementInput` (`KismetMathLibrary.MakeVector` _returnvalue_x_5 0.0 _returnvalue_z_3) (* 3 (* (`self.Distance`) 0.001)))
          (else
            (`self.AddMovementInput` (`KismetMathLibrary.MakeVector` _returnvalue_x_5 0.0 _returnvalue_z_3) 0.1)))))))

(fn `UserConstructionScript`)