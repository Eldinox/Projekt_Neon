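; Bob, the Paper2D player character: runs, double-jumps, dodges with a collision-profile swap, shoots, and fights with melee combos.
; Light/heavy inputs build a timed string of up to three hits, which ComboHandler maps by ground/air state to spawned attack actors and CharacterEnum.
; Tick turns that enum into flipbooks; only Normal of three switchable forms has attack logic.
; Also handles GameInstance health, HUD, death screen and BP_Camera zone triggers.
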(event `SetCooldnownAnimation`
  (params (Delay :type "Float (double-precision)"))
  ;[1 1 1] Cooldown for the Animations(wird nichtb verwendet)
  (set `self.UpdataAnimation` false)
  (`KismetSystemLibrary.Delay` Delay)
  (set `self.UpdataAnimation` true))

(event `InputAction|DashRight`
  (params (Key :type "Key Structure"))
  ;[1 1 1] Testing
  (:`Pressed`
    (`self.Dodge 2` true :!label _label)))

(event `self.ReceiveActorBeginOverlap`
  (params (OtherActor :type "Actor Object Reference"))
  ;[1 0 0.5664] Handle Overlap
  (`self.Handel Overlap` OtherActor))

(event `Key|Z`
  (params (Key :type "Key Structure"))
  ;[1 1 1] Testing
  (:`Pressed`
    (goto _label)))

(event `InputAction|DashLeft`
  (params (Key :type "Key Structure"))
  ;[1 1 1] Testing
  (:`Pressed`
    (`self.Dodge 2` false :!label _label_2)))

(event `UpdateAnimation`
  (bind _sprite (`self.Sprite`))
  (bind _returnvalue (`PaperFlipbookComponent.GetFlipbookLength` (`self.Sprite`)))
  (bind _returnvalue_2 (> (`KismetMathLibrary.VSize` (`self.GetVelocity`)) 0.0))
  ;[1 1 1] Handle Animation
  (switch `int` (`self.BobsForm`)
    (:`0`
      ;;[1 1 1] Switch Animation
      (if (`self.UpdataAnimation`)
        (switch `/Game/2DSideScroller/Extras/Enum_CharacterAnimation` (`self.CharacterEnum`)
          (:`NewEnumerator0`
            (if _returnvalue_2
              (if (not (`AudioComponent.IsPlaying` (stale _returnvalue_3)))
                (bind _returnvalue_3 (`GameplayStatics.SpawnSoundAttached` "/Game/Sounds/Bob/107624__stintx__running-02.107624__stintx__running-02" (`self.CapsuleComponent`))))
              (else
                (`AudioComponent.Stop` _returnvalue_3)))
            ;;[1 1 1] Select Flipbook
            (`PaperFlipbookComponent.SetFlipbook` (`self.Sprite`) (select `bool` _returnvalue_2 :`false` "/Game/2DSideScroller/Sprites/IdleBob/bobo_idle.bobo_idle" :`true` "/Game/2DSideScroller/Sprites/Animations/BobRUn/BobRun.BobRun" :!type "PaperFlipbook Object Reference")))
          (:`NewEnumerator1`
            (`AudioComponent.Stop` _returnvalue_3)
            (`PaperFlipbookComponent.SetFlipbook` _sprite "/Game/2DSideScroller/Sprites/Animations/BobJump/Jump.Jump"))
          (:`NewEnumerator2`
            (`AudioComponent.Stop` _returnvalue_3)
            (set `self.UpdataAnimation` false)
            (`PaperFlipbookComponent.SetFlipbook` (`self.Sprite`) "/Game/2DSideScroller/Sprites/Animations/Dolche/Dolche.Dolche" :!label _label_3)
            (`KismetSystemLibrary.Delay` _returnvalue :!label _label_4)
            (set `self.UpdataAnimation` true)
            (set `self.CharacterEnum` "NewEnumerator0"))
          (:`NewEnumerator3`
            (set `self.UpdataAnimation` false)
            (goto _label_3))
          (:`NewEnumerator6`
            (`AudioComponent.Stop` _returnvalue_3)
            (set `self.UpdataAnimation` false)
            (`PaperFlipbookComponent.SetFlipbook` (`self.Sprite`) "/Game/2DSideScroller/Sprites/Animations/Schlag/Schlag.Schlag" :!label _label_5)
            (goto _label_4))
          (:`NewEnumerator7`
            (set `self.UpdataAnimation` false)
            (goto _label_5))
          (:`NewEnumerator8`
            (set `self.UpdataAnimation` false)
            (`PaperFlipbookComponent.SetFlipbook` (`self.Sprite`) "/Game/2DSideScroller/Sprites/Animations/SpeedDolche/SpeedDolche.SpeedDolche")
            (goto _label_4))
          (:`NewEnumerator9`
            (set `self.UpdataAnimation` false)
            (`PaperFlipbookComponent.SetFlipbook` (`self.Sprite`) "/Game/2DSideScroller/Sprites/Animations/SpartaKick/SpartaKick.SpartaKick")
            (goto _label_4))
          (:`NewEnumerator10`
            (set `self.UpdataAnimation` false)
            (`PaperFlipbookComponent.SetFlipbook` (`self.Sprite`) "/Game/2DSideScroller/Sprites/Animations/DolcheUnten/DolcheUnten.DolcheUnten" :!label _label_6)
            (goto _label_4))
          (:`NewEnumerator11`
            (set `self.UpdataAnimation` false)
            (goto _label_6))
          (:`NewEnumerator12`
            (set `self.UpdataAnimation` false)
            (`PaperFlipbookComponent.SetFlipbook` (`self.Sprite`) "/Game/2DSideScroller/Sprites/Animations/DropKick/DropKick.DropKick")
            (goto _label_4))
          (:`NewEnumerator13`
            (set `self.UpdataAnimation` false)
            (`PaperFlipbookComponent.SetFlipbook` (`self.Sprite`) "/Game/2DSideScroller/Sprites/Animations/Uppercut/Uppercut.Uppercut")
            (goto _label_4))
          (:`NewEnumerator14`
            ;;[1 1 1] Jumping
            (set `self.UpdataAnimation` false)
            (`KismetSystemLibrary.PrintString` "sefsfsdfdsfsd")
            (`/Engine/EditorBlueprintResources/StandardMacros.DoOnce` false :!label _label_7
              (:`Completed`
                (`PaperFlipbookComponent.SetFlipbook` (`self.Sprite`) "/Game/2DSideScroller/Sprites/Animations/BobFlip/pushdown.pushdown")
                (`KismetSystemLibrary.Delay` _returnvalue)
                (set `self.UpdataAnimation` true)
                (set `self.CharacterEnum` "NewEnumerator0")
                (goto _label_7 :!via `Reset`))))
          (:`NewEnumerator15`
            (`/Engine/EditorBlueprintResources/StandardMacros.DoOnce` false :!label _label_8
              (:`Completed`
                (bind _returnvalue_4 (`PaperFlipbookComponent.SetFlipbook` _sprite "/Game/2DSideScroller/Sprites/Animations/BobFlip/Flip.Flip"))
                (`/Engine/EditorBlueprintResources/StandardMacros.DoOnce` false :!via `Reset` :!label _label_9
                  (:`Completed`
                    (`PaperFlipbookComponent.SetFlipbook` (`self.Sprite`) "/Game/2DSideScroller/Sprites/Animations/Fallen4/fallen4.fallen4" :!label _label_10)
                    (`KismetSystemLibrary.PrintString` "falle"))))))
          (:`NewEnumerator16`
            (if (not _returnvalue_4)
              (goto _label_10)))
          (:`NewEnumerator17`
            (goto _label_5)))))
    (:`1`
      (`PaperFlipbookComponent.SetFlipbook` (`self.Sprite`) "/Game/2DSideScroller/Sprites/EnemyTextures/Bob_Damage_Kopie_Flipbook.Bob_Damage_Kopie_Flipbook"))
    (:`2`
      (`PaperFlipbookComponent.SetFlipbook` (`self.Sprite`) "/Game/2DSideScroller/Sprites/EnemyTextures/Bob_Ranger_Kopie_Flipbook.Bob_Ranger_Kopie_Flipbook"))))

(event `Key|T`
  (params (Key :type "Key Structure"))
  ;[1 1 1] Testing
  (:`Pressed`
    (goto _label_2)))

(event `Dodge`
  (params (right :type Boolean))
  (bind _returnvalue (`NavMovementComponent.IsFalling` (`self.CharacterMovement`)))
  (bind _x (.x (`SceneComponent.GetComponentVelocity` (`self.RootComponent`))))
  ;[1 1 1] Testing
  (if (`self.CanDodge`)
    (`PrimitiveComponent.SetCollisionEnabled` (`self.CapsuleComponent`) "PhysicsOnly")
    (`MovementComponent.SetPlaneConstraintAxisSetting` (`self.CharacterMovement`) "Z")
    (if right
      (if _returnvalue
        (`self.LaunchCharacter` (`KismetMathLibrary.MakeVector` (- 1000.0 _x)))
        (else
          (`self.LaunchCharacter` (1000.0 0.0 0.0))))
      (elif _returnvalue
        (`self.LaunchCharacter` (`KismetMathLibrary.MakeVector` (- -1000.0 _x)))
        (else
          (`self.LaunchCharacter` (-1000.0 0.0 0.0)))))
    (set `self.CanDodge` false)
    (`KismetSystemLibrary.Delay` 0.4)
    (set `self.CanDodge` true)
    (`PrimitiveComponent.SetCollisionEnabled` (`self.CapsuleComponent`) "QueryAndPhysics")
    (`MovementComponent.SetPlaneConstraintAxisSetting` (`self.CharacterMovement`) "UseGlobalPhysicsSetting")))

(event `self.OnLanded`
  (params (Hit :type "HitResult Structure (by ref)"))
  ;[1 1 1] Handle Animation
  ;;[1 1 1] Jumping
  (set `self.CharacterEnum` "NewEnumerator0")
  (`GameplayStatics.SpawnSoundAttached` "/Game/Sounds/Bob/363922__kfatehi__land.363922__kfatehi__land" (`self.CapsuleComponent`))
  (`|ExecutionSequence`
    (:`then_0`
      (goto _label_8 :!via `Reset`))
    (:`then_1`
      (goto _label_9 :!via `Reset`))))

(event `InputAction|MeleeLeicht`
  (params (Key :type "Key Structure"))
  ;[1 1 1] Handle Animation
  ;;[1 1 1] Light Attack
  (:`Pressed`
    (if (not (`self.IsAttacking`))
      (`self.Cobo Handler` "L"))))

(event `InputAction|MeleeHard`
  (params (Key :type "Key Structure"))
  ;[1 1 1] Handle Animation
  ;;[1 1 1] Hard Attack
  (:`Pressed`
    (if (not (`self.IsAttacking`))
      (`self.Cobo Handler` "S"))))

(event `Tot`
  (bind _returnvalue (`GameplayStatics.GetPlayerController` 0))
  ;[0 0 0] Death
  (bind _returnvalue_2 (`|CreateWidget` "/Game/Blueprints/Bob/DeathScreen.DeathScreen_C" _returnvalue))
  (`UserWidget.AddToViewport` _returnvalue_2 0)
  (`self.DisableInput` null)
  (`WidgetBlueprintLibrary.SetInputMode_UIOnlyEx` _returnvalue _returnvalue_2)
  (set `PlayerController.bShowMouseCursor` true _returnvalue))

(event `self.ReceiveAnyDamage`
  (params (Damage :type "Float (single-precision)") (DamageType :type "DamageType Object Reference") (InstigatedBy :type "Controller Object Reference") (DamageCauser :type "Actor Object Reference"))
  (bind _returnvalue (`self.K2_GetActorLocation`))
  (bind _returnvalue_2 (`self.K2_GetActorRotation`))
  ;[1 1 1] Handle Animation
  ;;[1 1 1] Damage
  (bind _asmygame_instance (cast `/Game/Blueprints/MYGameInstance` (`GameplayStatics.GetGameInstance`)))
  (bind _output_get (set `/Game/Blueprints/MYGameInstance.PlayerHealth` (- (`/Game/Blueprints/MYGameInstance.PlayerHealth` _asmygame_instance) Damage) _asmygame_instance))
  (`self.updateHealthbar`)
  (switch `int` (`KismetMathLibrary.RandomInteger` 4)
    (:`0`
      (`GameplayStatics.SpawnEmitterAtLocation` "/Game/InfinityBladeEffects/Effects/HitSparkEnemy1.HitSparkEnemy1" _returnvalue _returnvalue_2))
    (:`1`
      (`GameplayStatics.SpawnEmitterAtLocation` "/Game/InfinityBladeEffects/Effects/HitSparkEnemy2.HitSparkEnemy2" _returnvalue _returnvalue_2))
    (:`2`
      (`GameplayStatics.SpawnEmitterAtLocation` "/Game/InfinityBladeEffects/Effects/HitSparkEnemy3.HitSparkEnemy3" _returnvalue _returnvalue_2))
    (:`3`
      (`GameplayStatics.SpawnEmitterAtLocation` "/Game/InfinityBladeEffects/Effects/HitSparkEnemy4.HitSparkEnemy4" _returnvalue _returnvalue_2)))
  (if (<= _output_get 0.0)
    (`self.Tot`)))

(event `Dodge 2`
  (params (right :type Boolean))
  (bind _returnvalue_x (`KismetMathLibrary.BreakVector` (`self.GetVelocity`)))
  ;[1 1 1] Testing
  (if (`self.CanDodge`)
    (`GameplayStatics.SpawnSoundAttached` "/Game/Sounds/Bob/NFF-ninja-move.NFF-ninja-move" (`self.CapsuleComponent`) "None" (0.0 0.0 0.0) (struct) "KeepRelativeOffset" false 0.2 2.5)
    (set `self.CanDodge` false)
    (`PrimitiveComponent.SetCollisionProfileName` (`self.CapsuleComponent`) "PlayerDodge")
    (`MovementComponent.SetPlaneConstraintAxisSetting` (`self.CharacterMovement`) "Y")
    (set `MovementComponent.Velocity` (0.0 0.0 0.0) (`self.CharacterMovement`))
    (set `CharacterMovementComponent.GravityScale` 0.0 (`self.CharacterMovement`))
    (if right
      (`self.LaunchCharacter` (2000.0 0.0 0.0))
      (`KismetSystemLibrary.Delay` 0.15)
      (if (not (<= _returnvalue_x 1000.0))
        (`self.LaunchCharacter` (-1000.0 0.0 0.0)))
      (else
        (`self.LaunchCharacter` (-2000.0 0.0 0.0))
        (`KismetSystemLibrary.Delay` 0.15)
        (if (not (>= _returnvalue_x -1000.0))
          (`self.LaunchCharacter` (1000.0 0.0 0.0)))))
    (`MovementComponent.SetPlaneConstraintAxisSetting` (`self.CharacterMovement`) "UseGlobalPhysicsSetting")
    (`PrimitiveComponent.SetCollisionProfileName` (`self.CapsuleComponent`) "Player")
    (set `CharacterMovementComponent.GravityScale` 2.0 (`self.CharacterMovement`))
    (`MovementComponent.SetPlaneConstraintAxisSetting` (`self.CharacterMovement`) "Y")
    (`KismetSystemLibrary.Delay` (`self.DodgeCooldown`))
    (set `self.CanDodge` true)
    (else
      (`KismetSystemLibrary.PrintString` "false"))))

(event `self.ReceiveBeginPlay`
  (bind _returnvalue (`GameplayStatics.GetPlayerController` 0))
  (bind _gamecamera (`self.GameCamera`))
  ;[1 1 1] Start
  (`|ExecutionSequence`
    (:`then_0`
      (`ActorComponent.SetIsReplicated` (`self.Sprite`) true))
    (:`then_1`
      (bind _returnvalue_2 (`|CreateWidget` "/Game/Blueprints/Bob/MainUI.MainUI_C" (`GameplayStatics.GetPlayerController` 0)))
      (set `self.UI` _returnvalue_2)
      (`UserWidget.AddToViewport` _returnvalue_2 0)
      (set `self.UpdataAnimation` true)
      (set `PlayerController.bShowMouseCursor` false _returnvalue)
      (`WidgetBlueprintLibrary.SetFocusToGameViewport`)
      (`WidgetBlueprintLibrary.SetInputMode_GameAndUIEx` _returnvalue))
    (:`then_2`
      (`self.updateHealthbar`))
    (:`then_3`
      ;[1 1 1] Set Camera
      (`self.Set Canera Reference`)
      (`/Game/Blueprints/Bob/Camera/Triggers/BP_CameraZone.SetCameraTarget` _gamecamera (`ActorComponent.GetOwner` (`self.CapsuleComponent`)))
      (`PlayerController.SetViewTargetWithBlend` (`GameplayStatics.GetPlayerController` 0) _gamecamera 0.0 "VTBlend_Linear" 0.0 false))))

(event `self.ReceiveTick`
  (params (DeltaSeconds :type "Float (single-precision)"))
  (bind _characterenum (`self.CharacterEnum`))
  (bind _charactermovement (`self.CharacterMovement`))
  (bind (_velocity_x _velocity_y _velocity_z) (`KismetMathLibrary.BreakVector` (`MovementComponent.Velocity` _charactermovement)))
  ;[1 1 1] Handle movement
  ;[1 1 1] Tick - Updates animation
  (if (and (`NavMovementComponent.IsFalling` _charactermovement) (< _velocity_z 0.0) (or (`|EnumEquality` _characterenum "NewEnumerator0") (`|EnumEquality` _characterenum "NewEnumerator1") (`|EnumEquality` _characterenum "NewEnumerator15") (`|EnumEquality` _characterenum "NewEnumerator16")))
    (set `self.CharacterEnum` "NewEnumerator16"))
  (`self.UpdateAnimation`)
  (`/Engine/EditorBlueprintResources/StandardMacros.CompareFloat` (.x (`MovementComponent.Velocity` (`self.GetMovementComponent`)))
    (:`>`
      (`self.K2_SetActorRotation` (struct) :!label _label_11))
    (:`==`
      (if (`self.bisMovingRight`)
        (goto _label_11)
        (else
          (`self.K2_SetActorRotation` (struct :`Yaw` -180.0) :!label _label_12))))
    (:`<`
      (goto _label_12))))

(event `InputAction|Shoot`
  (params (Key :type "Key Structure"))
  ;[1 1 1] Testing
  (:`Pressed`
    (if (`self.CanShoot`) :!label _label_13
      (set `self.CanShoot` false)
      (set `self.CharacterEnum` "NewEnumerator17")
      (bind _returnvalue (`|SpawnActorFromClass` "/Game/Blueprints/Bob/Attack_BP/Bob_Shoot.Bob_Shoot_C" (`SceneComponent.K2_GetComponentToWorld` (`self.Arrow1`)) "AdjustIfPossibleButAlwaysSpawn" "OverrideRootScale" null null))
      (`/Game/Blueprints/Bob/Default_Attack.Init` _returnvalue)
      (`GameplayStatics.SpawnSoundAttached` "/Game/Sounds/Bob/105016__julien-matthey__jm-fx-fireball-01.105016__julien-matthey__jm-fx-fireball-01" (`self.CapsuleComponent`) "None" (0.0 0.0 0.0) (struct) "KeepRelativeOffset" false 0.3)
      (`KismetSystemLibrary.Delay` 4.0)
      (set `self.CharacterEnum` "NewEnumerator0")
      (set `self.CanShoot` true))))

(event `InputAxis|MoveRight`
  (params (AxisValue :type "Float (single-precision)"))
  ;[1 1 1] Handle movement
  (if (> AxisValue 0.0)
    (set `self.bisMovingRight` true)
    (elif (< AxisValue 0.0)
      (set `self.bisMovingRight` false)))
  (`self.MakeNoise` 1.0)
  (`self.AddMovementInput` (1.0 0.0 0.0) AxisValue))

(event `Key|K`
  (params (Key :type "Key Structure"))
  ;[1 1 1] Testing
  (:`Pressed`
    (goto _label_13)))

(event `updateHealthbar`
  ;[0.375 0.01471 0] healthChange
  (bind _asmygame_instance (cast `/Game/Blueprints/MYGameInstance` (`GameplayStatics.GetGameInstance`)))
  (bind _asmain_ui (cast `/Game/Blueprints/Bob/MainUI` (`self.UI`)))
  (`ProgressBar.SetPercent` (`/Game/Blueprints/Bob/MainUI.ProgressBar_75` _asmain_ui) (/ (`/Game/Blueprints/MYGameInstance.PlayerHealth` _asmygame_instance) (`/Game/Blueprints/MYGameInstance.MaxPlayerHealth` _asmygame_instance))))

(event `InputAction|Jump`
  (params (Key :type "Key Structure"))
  (bind _capsulecomponent (`self.CapsuleComponent`))
  ;[1 1 1] Handle Jump
  (:`Pressed`
    (`self.Jump`)
    (switch `int` (`self.JumpCurrentCount`)
      (:`0`
        (`GameplayStatics.SpawnSoundAttached` "/Game/Sounds/Bob/380471__acebrian__jump.380471__acebrian__jump" _capsulecomponent)
        (set `self.CharacterEnum` "NewEnumerator1"))
      (:`1`
        (`GameplayStatics.SpawnSoundAttached` "/Game/Sounds/Bob/380471__acebrian__jump.380471__acebrian__jump" _capsulecomponent)
        (set `self.CharacterEnum` "NewEnumerator15"))))
  (:`Released`
    (`self.StopJumping`)))

(event `Cobo Handler`
  (params (Combo :type String))
  ;[1 1 1] Combo
  (set `self.ComboTime` 1.5)
  (set `self.ComboSring` (`KismetStringLibrary.Concat_StrStr` (`self.ComboSring`) Combo))
  (if (`self.ComboIsActive`)
    (`self.ComboHandler` (`self.ComboSring`))
    (else
      (set `self.ComboIsActive` true)
      (`self.ComboHandler` (`self.ComboSring`))
      (`KismetSystemLibrary.K2_SetTimer` null "ComboTimer" 0.0167 true))))

(event `InputAction|ChangeFormLeft`
  (params (Key :type "Key Structure"))
  ;[1 1 1] Change Form
  (:`Pressed`
    (bind _output_get (set `self.BobsForm` (- (`self.BobsForm`) 1)))
    (if (< _output_get 0)
      (set `self.BobsForm` 2))))

(event `InputAction|ChangeFormRight`
  (params (Key :type "Key Structure"))
  ;[1 1 1] Change Form
  (:`Pressed`
    (set `self.BobsForm` (mod (+ (`self.BobsForm`) 1) 3))))

(fn `ComboHandler`
  (params (ComboString :type String))
  (bind _returnvalue (`self.GetTransform`))
  (bind _returnvalue_2 (`self.GetTransform`))
  (bind _bobsform (`self.BobsForm`))
  ;[0.3854 0.3854 0.3854] Comment
  (set `self.ComboStringLength` (`KismetStringLibrary.Len` ComboString))
  (if (`NavMovementComponent.IsFalling` (`self.CharacterMovement`))
    (switch `int` _bobsform
      (:`0`
        ;[0.06097 1 0] Form1 Normal
        (switch `int` (`self.ComboStringLength`)
          (:`1`
            (switch `string` (`local.ComboString`)
              (:`L`
                (set `self.CharacterEnum` "NewEnumerator3" :!label _label)
                (bind _returnvalue_3 (`|SpawnActorFromClass` "/Game/Blueprints/Bob/Attack_BP/Attacks_Bob/Normal/NormalLightAttack.NormalLightAttack_C" _returnvalue "Undefined" "OverrideRootScale" null null))
                (`/Game/Blueprints/Bob/Default_Attack.Init` _returnvalue_3))
              (:`S`
                (set `self.CharacterEnum` "NewEnumerator7" :!label _label_2)
                (bind _returnvalue_4 (`|SpawnActorFromClass` "/Game/Blueprints/Bob/Attack_BP/Attacks_Bob/Normal/NormalHardAttack.NormalHardAttack_C" _returnvalue "Undefined" "OverrideRootScale" null null))
                (`/Game/Blueprints/Bob/Default_Attack.Init` _returnvalue_4))))
          (:`2`
            (switch `string` (`self.ComboSring`)
              (:`LL`
                (goto _label))
              (:`LS`
                (goto _label_2))
              (:`SL`
                (goto _label))
              (:`SS`
                (goto _label_2))))
          (:`3`
            (`|ExecutionSequence`
              (:`then_0`
                (switch `string` (`self.ComboSring`)
                  (:`LLL`
                    (goto _label))
                  (:`LLS`
                    (set `self.CharacterEnum` "NewEnumerator14")
                    (bind _returnvalue_5 (`|SpawnActorFromClass` "/Game/Blueprints/Bob/Attack_BP/Attacks_Bob/Normal/NormalPushdownAttack.NormalPushdownAttack_C" _returnvalue "Undefined" "OverrideRootScale" null null))
                    (`/Game/Blueprints/Bob/Default_Attack.Init` _returnvalue_5))
                  (:`LSL`
                    (goto _label))
                  (:`LSS`
                    (set `self.CharacterEnum` "NewEnumerator12")
                    (bind _returnvalue_6 (`|SpawnActorFromClass` "/Game/Blueprints/Bob/Attack_BP/Attacks_Bob/Normal/NormalAirPushbackAttack.NormalAirPushbackAttack_C" _returnvalue "Undefined" "OverrideRootScale" null null))
                    (`/Game/Blueprints/Bob/Default_Attack.Init` _returnvalue_6))
                  (:`SLL`
                    (goto _label))
                  (:`SLS`
                    (goto _label_2))
                  (:`SSL`
                    (goto _label))
                  (:`SSS`
                    (goto _label_2))))
              (:`then_1`
                ;[0.2865 0.03984 0] Stop Timer
                (set `self.ComboIsActive` false :!label _label_3)
                (set `self.ComboSring` "")
                (`KismetSystemLibrary.K2_ClearTimer` null "ComboTimer"))))))
      (:`1`
        ;[0 0.04508 1] Form2 Damage
        (switch `int` (`self.ComboStringLength`)
          (:`1`
            (switch `string` (`local.ComboString`)))
          (:`2`
            (switch `string` (`self.ComboSring`)))
          (:`3`
            (`|ExecutionSequence`
              (:`then_0`
                (switch `string` (`self.ComboSring`)))
              (:`then_1`
                (goto _label_3))))))
      (:`2`
        ;[1 0 0.01394] Form3 Range
        (switch `int` (`self.ComboStringLength`)
          (:`1`
            (switch `string` (`local.ComboString`)))
          (:`2`
            (switch `string` (`self.ComboSring`)))
          (:`3`
            (`|ExecutionSequence`
              (:`then_0`
                (switch `string` (`self.ComboSring`)))
              (:`then_1`
                (goto _label_3)))))))
    (else
      (switch `int` _bobsform
        (:`0`
          ;[0.06097 1 0] Form1 Normal
          (switch `int` (`self.ComboStringLength`)
            (:`1`
              (switch `string` (`local.ComboString`)
                (:`L`
                  (set `self.CharacterEnum` "NewEnumerator2" :!label _label_4)
                  (bind _returnvalue_7 (`|SpawnActorFromClass` "/Game/Blueprints/Bob/Attack_BP/Attacks_Bob/Normal/NormalFastAttack.NormalFastAttack_C" _returnvalue_2 "Undefined" "OverrideRootScale" null null))
                  (`/Game/Blueprints/Bob/Default_Attack.Init` _returnvalue_7))
                (:`S`
                  (set `self.CharacterEnum` "NewEnumerator6" :!label _label_5)
                  (bind _returnvalue_8 (`|SpawnActorFromClass` "/Game/Blueprints/Bob/Attack_BP/Attacks_Bob/Normal/NormalSlowAttack.NormalSlowAttack_C" _returnvalue_2 "Undefined" "OverrideRootScale" null null))
                  (`/Game/Blueprints/Bob/Default_Attack.Init` _returnvalue_8))))
            (:`2`
              (switch `string` (`self.ComboSring`)
                (:`LL`
                  (goto _label_4))
                (:`LS`
                  (set `self.CharacterEnum` "NewEnumerator10")
                  (bind _returnvalue_9 (`|SpawnActorFromClass` "/Game/Blueprints/Bob/Attack_BP/Attacks_Bob/Normal/NormalStackAttack.NormalStackAttack_C" _returnvalue_2 "Undefined" "OverrideRootScale" null null))
                  (`/Game/Blueprints/Bob/Default_Attack.Init` _returnvalue_9))
                (:`SL`
                  (goto _label_4))
                (:`SS`
                  (goto _label_5))))
            (:`3`
              (`|ExecutionSequence`
                (:`then_0`
                  (switch `string` (`self.ComboSring`)
                    (:`LLL`
                      (set `self.CharacterEnum` "NewEnumerator8")
                      (bind _returnvalue_10 (`|SpawnActorFromClass` "/Game/Blueprints/Bob/Attack_BP/Attacks_Bob/Normal/NormalLotLightAttacks.NormalLotLightAttacks_C" _returnvalue_2 "Undefined" "OverrideRootScale" null null))
                      (`/Game/Blueprints/Bob/Default_Attack.Init` _returnvalue_10))
                    (:`LLS`
                      (set `self.CharacterEnum` "NewEnumerator13")
                      (bind _returnvalue_11 (`|SpawnActorFromClass` "/Game/Blueprints/Bob/Attack_BP/Attacks_Bob/Normal/NormalUppercutAttack.NormalUppercutAttack_C" _returnvalue_2 "Undefined" "OverrideRootScale" null null))
                      (`/Game/Blueprints/Bob/Default_Attack.Init` _returnvalue_11))
                    (:`LSL`
                      (goto _label_4))
                    (:`LSS`
                      (set `self.CharacterEnum` "NewEnumerator11")
                      (bind _returnvalue_12 (`|SpawnActorFromClass` "/Game/Blueprints/Bob/Attack_BP/Attacks_Bob/Normal/NormalStackWideAttack.NormalStackWideAttack_C" _returnvalue_2 "Undefined" "OverrideRootScale" null null))
                      (`/Game/Blueprints/Bob/Default_Attack.Init` _returnvalue_12))
                    (:`SLL`
                      (goto _label_4))
                    (:`SLS`
                      (goto _label_5))
                    (:`SSL`
                      (goto _label_4))
                    (:`SSS`
                      (set `self.CharacterEnum` "NewEnumerator9")
                      (bind _returnvalue_13 (`|SpawnActorFromClass` "/Game/Blueprints/Bob/Attack_BP/Attacks_Bob/Normal/NormalPushbackAttack.NormalPushbackAttack_C" _returnvalue_2 "Undefined" "OverrideRootScale" null null))
                      (`/Game/Blueprints/Bob/Default_Attack.Init` _returnvalue_13))))
                (:`then_1`
                  (goto _label_3))))))
        (:`1`
          ;[0 0.04508 1] Form2 Damage
          (switch `int` (`self.ComboStringLength`)
            (:`1`
              (switch `string` (`local.ComboString`)))
            (:`2`
              (switch `string` (`self.ComboSring`)))
            (:`3`
              (`|ExecutionSequence`
                (:`then_0`
                  (switch `string` (`self.ComboSring`)))
                (:`then_1`
                  (goto _label_3))))))
        (:`2`
          ;[1 0 0.01394] Form3 Range
          (switch `int` (`self.ComboStringLength`)
            (:`1`
              (switch `string` (`local.ComboString`)))
            (:`2`
              (switch `string` (`self.ComboSring`)))
            (:`3`
              (`|ExecutionSequence`
                (:`then_0`
                  (switch `string` (`self.ComboSring`)))
                (:`then_1`
                  (goto _label_3))))))))))

(fn `ComboTimer`
  (set `self.ComboTime` (`KismetMathLibrary.FClamp` (- (`self.ComboTime`) 0.0167) 0.0 10.0))
  (if (== (`self.ComboTime`) 0.0)
    (set `self.ComboIsActive` false)
    (set `self.ComboSring` "")
    (`KismetSystemLibrary.K2_ClearTimer` null "ComboTimer")))

(fn `Handel Overlap`
  (params (Object :type "Actor Object Reference"))
  (bind _returnvalue (`KismetSystemLibrary.GetDisplayName` Object))
  (if (`KismetStringLibrary.StartsWith` _returnvalue "TCameraZone")
    (`/Game/Blueprints/Bob/Camera/Triggers/BP_CameraZone.OnCameraTrigger` (`self.GameCamera`) _returnvalue)))

(fn `Set Canera Reference`
  (bind _outactors (`GameplayStatics.GetAllActorsOfClass` "/Game/Blueprints/Bob/Camera/BP_Camera.BP_Camera_C"))
  (bind _asbp_camera (cast `/Game/Blueprints/Bob/Camera/BP_Camera` (`|GetArrayItem` _outactors))
    (:`then`
      (set `self.GameCamera` _asbp_camera))
    (:`CastFailed`
      (`KismetSystemLibrary.PrintString` "Konnte Camera Reference nicht setzten"))))

(fn `SetIsAttacking`
  (params (setAttacking :type Boolean))
  (set `self.IsAttacking` setAttacking))

(fn `UserConstructionScript`)