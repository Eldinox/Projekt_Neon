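; Attack hitbox actor that sweeps a box along a short path relative to the player character, Bob.
; BeginPlay sizes the box, mirrors the travel vector for Bob's facing and scales a timeline to the configured duration.
; Each update re-anchors the path to Bob's position and current facing side, then lerps along it.
; On finish it clears hits, resets collision and replays until Count runs out, then destroys itself.
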(event `self.ReceiveBeginPlay`
  (bind (_offset_x _offset_y _offset_z) (`KismetMathLibrary.BreakVector` (`self.Offset`)))
  (bind _boxextent_x (`KismetMathLibrary.BreakVector` (`BoxComponent.BoxExtent` (`self.Box`))))
  (bind _returnvalue (+ _offset_x _boxextent_x))
  (`BoxComponent.SetBoxExtent` (`self.Box`) (`self.BoxExtents`) true)
  (bind _asbob (cast `/Game/Blueprints/Bob/Bob` (`GameplayStatics.GetPlayerCharacter` 0)))
  (if (not (`/Game/Blueprints/Bob/Bob.bisMovingRight` _asbob))
    (set `self.MoveSpace` (`KismetMathLibrary.MakeVector` (* (.x (`self.MoveSpace`)) -1.0) (.y (`self.MoveSpace`)) (.z (`self.MoveSpace`)))))
  (`TimelineComponent.SetPlayRate` (`self.Move_Stuff`) (`KismetMathLibrary.MultiplyMultiply_FloatFloat` (`self.PlayRateInSec`) -1.0))
  (bind (_direction _alpha) (`Timeline|Move_Stuff` :!via `PlayFromStart` :!label _label)
    (:`Update`
      (bind _asbob_2 (cast `/Game/Blueprints/Bob/Bob` (`GameplayStatics.GetPlayerCharacter` 0)))
      (if (`/Game/Blueprints/Bob/Bob.bisMovingRight` _asbob_2)
        (bind (_returnvalue_x _returnvalue_y _returnvalue_z) (`KismetMathLibrary.BreakVector` (`SceneComponent.K2_GetComponentLocation` (`Actor.RootComponent` _asbob_2))))
        (bind _output_get (set `self.setLocation` (`KismetMathLibrary.MakeVector` (+ _returnvalue_x _returnvalue) _returnvalue_y (+ _returnvalue_z _offset_z))))
        (set `self.destination` (+ _output_get (`self.MoveSpace`)))
        (else
          (bind _output_get_2 (set `self.setLocation` (`KismetMathLibrary.MakeVector` (- _returnvalue_x _returnvalue) _returnvalue_y (+ _returnvalue_z _offset_z))))
          (set `self.destination` (+ _output_get_2 (`self.MoveSpace`)))))
      (`self.K2_SetActorLocation` (`KismetMathLibrary.VLerp` (`self.setLocation`) (`self.destination`) _alpha)))
    (:`Finished`
      (bind _again (`self.Again`))
      (if _again
        (`self.ClearHitList`)
        (`self.ResetCollision`)
        (goto _label :!via `PlayFromStart`)
        (else
          (`self.K2_DestroyActor`))))))

(fn `Again`
  (returns (Again :type Boolean))
  (bind _output_get (set `self.Count` (- (`self.Count`) 1)))
  (if (== _output_get 0)
    (return false)
    (else
      (return true))))

(fn `UserConstructionScript`)