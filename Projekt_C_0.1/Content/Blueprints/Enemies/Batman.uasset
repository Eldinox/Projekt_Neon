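; Flying bat enemy that patrols, chases and dive-attacks the player, with flapping and alert sounds.
; Each Tick updates the distance, derives a state enum from range and the Chasing/Attacking flags, runs Patroll, Chase or Attack, then calls FlyingUpAndDown.
; Attack launches the bat down toward the player's side on X, then holds a timed recovery that blocks further attacks and re-arms the chase sound's DoOnce.
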(event `self.ReceiveTick`
  (params (DeltaSeconds :type "Float (single-precision)"))
  (bind _enemystateenum (`self.EnemyStateEnum`))
  (`|ExecutionSequence`
    (:`then_0`
      ;[0.6565 1 0.555] 1. Distanzberechnung
      (`self.CalculateDistance`))
    (:`then_1`
      ;[0.4479 0.5155 1] 2. Setze Enum auf aktuellen Status
      (if (<= (`self.Distance`) 2000.0)
        (if (`self.Chasing`)
          (if (`self.Attacking`)
            (set `self.EnemyStateEnum` "NewEnumerator3")
            (if (not (`AudioComponent.IsPlaying` (stale _returnvalue))) :!label _label
              (bind _returnvalue (`GameplayStatics.SpawnSoundAttached` "/Game/Sounds/NFF-flapping.NFF-flapping" (`self.CapsuleComponent`) "None" (`SceneComponent.K2_GetComponentLocation` (`self.CapsuleComponent`)) (struct) "SnapToTargetIncludingScale" false 0.01)))
            (else
              (set `self.EnemyStateEnum` "NewEnumerator2")
              (`|ExecutionSequence`
                (:`then_0`
                  (goto _label))
                (:`then_1`
                  (`/Engine/EditorBlueprintResources/StandardMacros.DoOnce` false :!label _label_2
                    (:`Completed`
                      (`GameplayStatics.SpawnSoundAttached` "/Game/Sounds/Enemies/Bat/NFF-shooting-star-02.NFF-shooting-star-02" (`self.CapsuleComponent`) "None" (0.0 0.0 0.0) (struct) "KeepRelativeOffset" false 0.3)))))))
          (else
            (set `self.EnemyStateEnum` "NewEnumerator1")
            (goto _label)))
        (else
          (set `self.EnemyStateEnum` "NewEnumerator0"))))
    (:`then_2`
      ;[0.4479 0.5155 1] 3. Aktion je nach Enum Status
      (if (`|EnumEquality` _enemystateenum "NewEnumerator0")
        _
        (elif (`|EnumEquality` _enemystateenum "NewEnumerator1")
          (if (not (`self.Attacking`))
            (`self.Patroll`))
          (elif (`|EnumEquality` _enemystateenum "NewEnumerator2")
            (if (<= (`self.Distance`) 300.0)
              (`self.Attack`)
              (else
                (`self.Chase`)))))))
    (:`then_3`
      ;[0.302 0.5611 1] Flying Up And Down
      (`self.FlyingUpAndDown`))))

(event `Attack`
  (bind _returnvalue_x (`KismetMathLibrary.BreakVector` (`self.K2_GetActorLocation`)))
  (bind _returnvalue_x_2 (`KismetMathLibrary.BreakVector` (`self.K2_GetActorLocation` (`GameplayStatics.GetPlayerCharacter` 0))))
  ;[1 0.6146 0.6146] Attack
  (`|ExecutionSequence`
    (:`then_1`
      (if (not (or (`self.Recovering`) (`self.Attacking`)))
        (set `self.Chasing` false)
        (set `self.Attacking` true)
        (if (>= _returnvalue_x_2 _returnvalue_x)
          (`self.LaunchCharacter` (300.0 0.0 -200.0))
          (else
            (`self.LaunchCharacter` (-300.0 0.0 -200.0))))
        (`KismetSystemLibrary.Delay` 0.4)
        (`GameplayStatics.SpawnSoundAttached` "/Game/Sounds/NFF-suck.NFF-suck" (`self.CapsuleComponent`) "None" (0.0 0.0 0.0) (struct) "KeepRelativeOffset" false 0.2)
        (set `self.Recovering` true)
        (set `self.Attacking` false)
        (set `self.Chasing` true)
        (`KismetSystemLibrary.Delay` 3.0)
        (set `self.Recovering` false)
        (goto _label_2 :!via `Reset`)))))

(fn `UserConstructionScript`
  (`parent.UserConstructionScript`))