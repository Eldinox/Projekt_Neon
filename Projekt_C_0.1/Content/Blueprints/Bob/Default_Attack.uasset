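; Default attack hitbox actor for Bob that damages overlapping "Enemy"-tagged actors, tracking AlreadyHit to prevent double hits.
; Optionally launches Default_Enemy targets, mirroring launch X by Bob's facing, captured at Init or read at hit time if unset.
; Init destroys it after LifeTime, first setting Bob's attacking flag if BockCombo is on; destruction clears that flag.
; ResetCollision toggles the box's collision and ClearHitList empties the hit list.
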(event `self.ReceiveDestroyed`
  (bind _asbob (cast `/Game/Blueprints/Bob/Bob` (`GameplayStatics.GetPlayerCharacter` 0)))
  (`/Game/Blueprints/Bob/Bob.SetIsAttacking` _asbob false))

(event `Init`
  (bind _lifetime (`self.lifeTime`))
  (bind _asbob (cast `/Game/Blueprints/Bob/Bob` (`GameplayStatics.GetPlayerCharacter` 0)))
  (if (`/Game/Blueprints/Bob/Bob.bisMovingRight` _asbob)
    (set `self.IsLaunchingRight` -1)
    (else
      (set `self.IsLaunchingRight` 1)))
  ;[1 1 1] lifeTime
  (if (`self.BockCombo`)
    (bind _asbob_2 (cast `/Game/Blueprints/Bob/Bob` (`GameplayStatics.GetPlayerCharacter` 0)))
    (`/Game/Blueprints/Bob/Bob.SetIsAttacking` _asbob_2 true)
    (`KismetSystemLibrary.PrintString` (`KismetStringLibrary.Conv_DoubleToString` _lifetime)))
  (`KismetSystemLibrary.Delay` _lifetime)
  (`self.K2_DestroyActor`))

(event `self.Box.OnComponentBeginOverlap`
  (params (OverlappedComponent :type "PrimitiveComponent Object Reference") (OtherActor :type "Actor Object Reference") (OtherComp :type "PrimitiveComponent Object Reference") (OtherBodyIndex :type Integer) (bFromSweep :type Boolean) (SweepResult :type "HitResult Structure (by ref)"))
  (bind _launchenemy (`self.LaunchEnemy`))
  ;[1 1 1] ApplyDamage
  (set `self.DoDamage` true)
  (bind _outactors (`GameplayStatics.GetAllActorsWithTag` "Enemy"))
  (for _array_element _outactors
    (if (== _array_element OtherActor)
      ;;[1 1 1] Verhindert einen doppelten hit
      (for _array_element_2 (`self.AlreadyHit`)
        (if (== OtherActor _array_element_2)
          (set `self.DoDamage` false)))
      (if (`self.DoDamage`)
        (`GameplayStatics.ApplyDamage` _array_element (`self.Damage`))
        (if (`self.IsLaunchEnemy`)
          (bind _asdefault_enemy (cast `/Game/Blueprints/Enemies/Default_Enemy` OtherActor))
          (set `MovementComponent.Velocity` (0.0 0.0 0.0) (`Character.CharacterMovement` _asdefault_enemy))
          (switch `int` (`self.IsLaunchingRight`)
            (:`-1`
              (`Character.LaunchCharacter` _asdefault_enemy _launchenemy false false :!label _label)
              (`KismetSystemLibrary.PrintString` "right"))
            (:`0`
              (bind _asbob (cast `/Game/Blueprints/Bob/Bob` (`GameplayStatics.GetPlayerCharacter` 0)))
              (if (`/Game/Blueprints/Bob/Bob.bisMovingRight` _asbob)
                (goto _label)
                (else
                  (`Character.LaunchCharacter` _asdefault_enemy (`KismetMathLibrary.MakeVector` (* (.x _launchenemy) -1.0) (.y _launchenemy) (.z _launchenemy)) false false :!label _label_2)
                  (`KismetSystemLibrary.PrintString` "left"))))
            (:`1`
              (goto _label_2))))
        (`KismetArrayLibrary.Array_Add` (`self.AlreadyHit`) OtherActor)))))

(event `ResetCollision`
  (bind _box (`self.Box`))
  ;[1 1 1] ApplyDamage
  (`PrimitiveComponent.SetCollisionEnabled` _box "NoCollision")
  (`PrimitiveComponent.SetCollisionEnabled` _box "QueryOnly"))

(fn `ClearHitList`
  (`KismetArrayLibrary.Array_Clear` (`self.AlreadyHit`)))

(fn `UserConstructionScript`)